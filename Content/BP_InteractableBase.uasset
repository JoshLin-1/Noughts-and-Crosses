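; Interactable cube that acts as a markable cell in what appears to be a circle-and-cross turn game, showing each mark by swapping materials.
; Circle and Cross set the mark material while Hi is true, and EndFocus restores the cube material until OnInteract clears Hi.
; The InClick variants apply a mark once by clearing EachTurn, which also gates StartFocus.
; BeginPlay caches a dynamic material's GlowColor, but the glow-changing nodes are disconnected.
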(event `InteractInterface.StartFocus`
  (if (== (`self.eachTurn`) true)
    (`parent.StartFocus`)))

(event `self.ReceiveBeginPlay`
  ;[1 1 1] Storing Colour Details
  (bind _returnvalue (`PrimitiveComponent.CreateDynamicMaterialInstance` (`self.Cube`) 0 null "None"))
  (bind _output_get (set `self.MaterialInstance` _returnvalue))
  (bind _returnvalue_2 (`MaterialInstanceDynamic.K2_GetVectorParameterValue` _output_get "GlowColor"))
  (set `self.DefaultColour` _returnvalue_2))

(event `InteractInterface.Circle`
  (if (== (`self.Hi`) true)
    (`PrimitiveComponent.SetMaterial` (`self.Cube`) 0 "/Game/MI_FlatWhite.MI_FlatWhite")))

(event `InteractInterface.CircleInClick`
  (if (== (`self.eachTurn`) true)
    (`PrimitiveComponent.SetMaterial` (`self.Cube`) 0 "/Game/MI_FlatWhite.MI_FlatWhite")
    (set `self.eachTurn` false)))

(event `InteractInterface.Cross`
  (if (== (`self.Hi`) true)
    (`PrimitiveComponent.SetMaterial` (`self.Cube`) 0 "/Game/MI_FlatWhite_2.MI_FlatWhite_2")))

(event `InteractInterface.CrossInClick`
  (if (== (`self.eachTurn`) true)
    (`PrimitiveComponent.SetMaterial` (`self.Cube`) 0 "/Game/MI_FlatWhite_2.MI_FlatWhite_2")
    (set `self.eachTurn` false)))

(event `InteractInterface.EndFocus`
  (`parent.EndFocus`)
  (if (== (`self.Hi`) true)
    (`PrimitiveComponent.SetMaterial` (`self.Cube`) 0 "/Engine/VREditor/BasicMeshes/MI_Cube_01.MI_Cube_01")))

(event `InteractInterface.OnInteract`
  (params (Caller :type "Actor Object Reference"))
  (`parent.OnInteract` null)
  (set `self.Hi` false))

(fn `UserConstructionScript`)